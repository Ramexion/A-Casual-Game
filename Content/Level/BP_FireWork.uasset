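; BP_FireWork is a level actor that sets off a firework effect for a player who has collected enough coins.
; When the player pawn enters its sphere, a DoOnce MultiInput gate lets through a check of the character's Coins against CoinsNeeded.
; Success activates the particle system and audio through UpdateFire.
; Failure loops back after a short delay into the same gate, which has no reset shown.
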(event OnComponentBeginOverlap(Sphere)
  (params (OverlappedComponent :type Primitive%20Component%20Object%20Reference) (OtherActor :type Actor%20Object%20Reference) (OtherComp :type Primitive%20Component%20Object%20Reference) (OtherBodyIndex :type Integer) (bFromSweep :type Boolean) (SweepResult :type Hit%20Result%20Structure%20%28by%20ref%29))
  (bind _returnvalue (Game|Player|GetPlayerPawn 0))
  (if (== OtherActor _returnvalue) :!label _label
    (bind _asbp_third_person_character (Utilities|Casting|CastToBP_ThirdPersonCharacter _returnvalue))
    (|DoOnceMultiInput
      (:A%20Out
        (if (>= (Variables|/Game/ThirdPerson/Blueprints/BP_ThirdPersonCharacter.BP_ThirdPersonCharacter_C|GetCoins _asbp_third_person_character) (Variables|Default|GetCoins%20Needed))
          (CallFunction|UpdateFire)
          (else
            (Utilities|FlowControl|Delay 1.0)
            (goto _label)))))))

(event Custom|Update%20Fire
  (Components|Activation|Activate (Variables|Default|GetParticleSystem) false)
  (Components|Activation|Activate (Variables|Default|GetAudio) false))

(event EventBeginPlay)

(event Collision|EventActorBeginOverlap
  (params (OtherActor :type Actor%20Object%20Reference)))

(event EventTick
  (params (DeltaSeconds :type Float%20%28single-precision%29)))

(fn ConstructionScript)